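; BP_Enemy is a cube enemy actor with a health bar widget, destroyed when the third-person character hits it.
; On BeginPlay it passes itself to the WB_HealthBar widget, and every Tick it rotates that widget to face the player's mesh.
; A character hit on the cube lowers Health, then always destroys the actor, as the branch is fixed true and the Health check is unconnected.
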(event `self.ReceiveBeginPlay`
  (bind _aswb_health_bar (cast `/Game/KelasUI2/WB_HealthBar` (`WidgetComponent.GetUserWidgetObject` (`self.Widget`))))
  (set `/Game/KelasUI2/WB_HealthBar.cube` self _aswb_health_bar))

(event `self.ReceiveTick`
  (params (DeltaSeconds :type "Float (single-precision)"))
  (bind _widget (`self.Widget`))
  (`SceneComponent.K2_SetWorldRotation` _widget (`KismetMathLibrary.FindLookAtRotation` (`SceneComponent.K2_GetComponentLocation` _widget) (`SceneComponent.K2_GetComponentLocation` (`Character.Mesh` (`GameplayStatics.GetPlayerCharacter` 0)))) false false))

(event `self.Cube.OnComponentHit`
  (params (HitComponent :type "PrimitiveComponent Object Reference") (OtherActor :type "Actor Object Reference") (OtherComp :type "PrimitiveComponent Object Reference") (NormalImpulse :type "Vector Structure") (Hit :type "HitResult Structure (by ref)"))
  (cast `/Game/ThirdPerson/Blueprints/BP_ThirdPersonCharacter` OtherActor)
  (set `self.Health` (- (`self.Health`) 5))
  (if true
    (`self.K2_DestroyActor`)))

(fn `UserConstructionScript`)