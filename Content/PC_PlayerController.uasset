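; Player controller that provides a debug line trace from the third-person character.
; On BeginPlay it caches the player's BP_ThirdPersonCharacter.
; Pressing the C debug key runs a persistent multi line trace on Visibility along the character's PlayerArrow forward vector and prints each hit actor's name.
; A single-hit line trace variant is present but disconnected.
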(event EventBeginPlay
  (bind _asbp_third_person_character (Utilities|Casting|CastToBP_ThirdPersonCharacter (Game|GetPlayerCharacter 0)))
  (Variables|Default|SetplayerCharacter _asbp_third_person_character))

(event EventTick
  (params (DeltaSeconds :type Float%20%28single-precision%29)))

(event Input|KeyboardEvents|DebugKeyC
  (params (Key :type Key%20Structure :default "None") (ActionValue :type Input%20Action%20Value%20Structure))
  (bind _playercharacter (Variables|Default|GetplayerCharacter))
  (bind _playerarrow (Variables|/Game/ThirdPerson/Blueprints/BP_ThirdPersonCharacter.BP_ThirdPersonCharacter_C|GetPlayerArrow _playercharacter))
  (bind _returnvalue (Transformation|GetWorldLocation _playerarrow))
  (:Pressed
    (bind _outhits (Collision|MultiLineTraceByChannel _returnvalue (+ _returnvalue (* (Math|Vector|GetForwardVector _playerarrow) 1e+03)) "TraceTypeQuery1" false 0 "Persistent"))
    (for _array_element _outhits
      (Development|PrintString (Utilities|GetDisplayName (.HitActor (Collision|BreakHitResult _array_element)))))))

(fn ConstructionScript)